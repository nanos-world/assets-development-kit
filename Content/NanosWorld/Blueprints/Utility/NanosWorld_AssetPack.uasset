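; Nanos World asset pack utility that builds a TOML-style config string from categorized lists of asset references.
; Per-category generators feed FetchAssetField, which derives keys and local paths, optionally loading static meshes to embed bounds.
; MakeFinalGeneratedString adds metadata, engine version and the detected game or plugin root folder, storing the result in Generated.
; Blueprint class paths lose their class suffix first; GenerateParticles actually runs the sounds generator.
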(fn CallAllGenerate
  (TOMLGeneration|Assets|Internal|InternalGenerateMaps)
  (TOMLGeneration|Assets|Internal|InternalGenerateBlueprints)
  (TOMLGeneration|Assets|Internal|InternalGenerateStaticMeshes)
  (TOMLGeneration|Assets|Internal|InternalGenerateSkeletalMeshes)
  (TOMLGeneration|Assets|Internal|InternalGenerateSounds)
  (TOMLGeneration|Assets|Internal|InternalGenerateParticles)
  (TOMLGeneration|Assets|Internal|InternalGenerateAnimations)
  (TOMLGeneration|Assets|Internal|InternalGenerateMaterials)
  (TOMLGeneration|Assets|Internal|InternalGenerateOthers)
  (return))

(fn FetchAssetField
  (params (assets :type Array%20of%20Object%20Soft%20Object%20References) (title :type String) (comment :type String))
  (if (not (Utilities|Array|IsEmpty assets))
    (for (_array_element _array_index) assets
      (if (Utilities|IsValidSoftObjectReference _array_element)
        (bind (_localpath _assetname) (Utility|GetLocalPathfromFullPath (Utilities|BreakSoftObjectPath (Class|KismetSystemLibrary|ToSoftObjPath(SoftObjRef) _array_element))))
        (LocalVariables|SetAssetsString (Utilities|String|Append (LocalVariables|GetAssetsString) "    " (Utilities|String|Append _assetname " = { path = \"" _localpath "\", key = \"" _assetname "\"" (TOMLGeneration|Assets|StaticMesh|TryGenerateStaticMeshBound _array_element (Variables|Meta|GetTitle)) " }") (Utilities|String|SelectString " 
" " 
    " (== (Utilities|Array|LastIndex assets) _array_index))))))
    (Variables|Default|SetFinalAssetString (Utilities|String|Append (Variables|Default|GetFinalAssetString) "" (Utilities|String|ToString(Text) (Utilities|Text|FormatText "    # {comment} 
    [assets.{title}] 
    {assets}" comment title (LocalVariables|GetAssetsString)))))
    (return)
    (else
      (return))))

(fn GetLocalPathfromFullPath
  (params (Path :type String))
  (bind _rights (Utilities|String|Split Path "/"))
  (bind (_lefts _rights_2) (Utilities|String|Split _rights "/"))
  (Variables|Default|SetUnreal_Root _lefts)
  (Variables|Default|SetUnreal_Folder (.LeftS (Utilities|String|Split _rights_2 "/")))
  (return (.LeftS (Utilities|String|Split (Utilities|String|SelectString (.RightS (Utilities|String|Split _rights_2 (Utilities|String|Append (Variables|Default|GetUnreal_Folder) "/"))) _rights_2 (Utilities|Enum|Equal(Enum) (Variables|Default|GetUnreal_Root) "Game")) "." "IgnoreCase" "FromEnd")) (.RightS (Utilities|String|Split (Utilities|String|SelectString (.RightS (Utilities|String|Split _rights_2 (Utilities|String|Append (Variables|Default|GetUnreal_Folder) "/"))) _rights_2 (Utilities|Enum|Equal(Enum) (Variables|Default|GetUnreal_Root) "Game")) "." "IgnoreCase" "FromEnd"))))

(fn GenerateBlueprintsArray
  (for _array_element (Variables|Assets|GetBlueprints)
    (Utilities|Array|Add (LocalVariables|GetOut) (Class|KismetSystemLibrary|ToSoftObjRef(SoftObjPath) (Utilities|MakeSoftObjectPath (.LeftS (Utilities|String|Split (Utilities|BreakSoftClassPath (Utilities|ToSoftClassPath _array_element)) "_" "IgnoreCase" "FromEnd"))))))
  (return (LocalVariables|GetOut)))

(fn MakeFinalGeneratedString
  (Variables|TOMLGeneration|SetGenerated (Utilities|String|ToString(Text) (Utilities|Text|FormatText "# vault configurations 
[meta] 
    # friendly name 
    title =                 \"{title}\" 
    # contributors 
    author =                \"{author}\" 
    # version 
    version =               \"{version}\" 
 
# asset pack configurations 
[asset_pack] 
    # asset packs requirements 
    assets_requirements = [ 
                             
    ] 
 
# unreal engine configurations 
[unreal] 
    # unreal engine folder - the exact name of the root folder inside Content/ or Plugin/ used in Unreal 
    unreal_folder =         \"{unreal_folder}\" 
    # unreal engine version - unreal version this asset pack was compiled on 
    unreal_version =        \"{unreal_version}\" 
    # whether this asset pack was created as a plugin content 
    is_plugin_content =     {is_plugin} 
 
# assets files 
[assets] 
{assets}" (Variables|Meta|GetTitle) (Variables|Meta|GetAuthor) (Variables|Meta|GetVersion) (select (not (Utilities|Enum|Equal(Enum) (Variables|Default|GetUnreal_Root) "Game")) (Variables|Default|GetUnreal_Root) (Variables|Default|GetUnreal_Folder)) (.LeftS (Utilities|String|Split (Development|GetEngineVersion) "-")) (not (Utilities|Enum|Equal(Enum) (Variables|Default|GetUnreal_Root) "Game")) (Variables|Default|GetFinalAssetString))))
  (Variables|Default|SetUnreal_Root "")
  (Variables|Default|SetUnreal_Folder "")
  (Variables|Default|SetFinalAssetString ""))

(fn InternalGenerateOthers
  (TOMLGeneration|Assets|FetchAssetField (Variables|Assets|GetOthers) "others" "others")
  (return))

(fn InternalGenerateStaticMeshes
  (TOMLGeneration|Assets|FetchAssetField (Variables|Assets|GetStaticMeshes) "static_meshes" "static meshes")
  (return))

(fn InternalGenerateSkeletalMeshes
  (TOMLGeneration|Assets|FetchAssetField (Variables|Assets|GetSkeletalMeshes) "skeletal_meshes" "skeletal meshes")
  (return))

(fn InternalGenerateSounds
  (TOMLGeneration|Assets|FetchAssetField (Variables|Assets|GetSounds) "sounds" "sounds")
  (return))

(fn InternalGenerateParticles
  (TOMLGeneration|Assets|FetchAssetField (Variables|Assets|GetParticles) "particles" "particles")
  (return))

(fn InternalGenerateAnimations
  (TOMLGeneration|Assets|FetchAssetField (Variables|Assets|GetAnimations) "animations" "animations")
  (return))

(fn InternalGenerateMaterials
  (TOMLGeneration|Assets|FetchAssetField (Variables|Assets|GetMaterials) "materials" "materials")
  (return))

(fn AddItemsArray
  (params (Array :type Array%20of%20Object%20Soft%20Object%20References) (Add :type Array%20of%20Object%20Soft%20Object%20References))
  (for _array_element Add
    (Utilities|Array|Add Array _array_element))
  (return))

(fn TryGenerateStaticMeshBound
  (params (Asset :type Object%20Soft%20Object%20Reference) (type :type String))
  (if (Variables|Settings|GetIncludeBoundsForStaticMeshes)
    (if (Utilities|Enum|Equal(Enum) type "static_meshes")
      (bind _returnvalue (Utilities|LoadAssetBlocking Asset))
      (bind _asstatic_mesh (Utilities|Casting|CastToStaticMesh _returnvalue)
        (:then
          (return (Utilities|String|Append ", bounds = { " (Utilities|String|Append "origin = \"" (CallFunction|FVectortoVectorString (.origin (StaticMesh|GetBounds _asstatic_mesh))) "\",") (Utilities|String|Append " box_extent = \"" (CallFunction|FVectortoVectorString (.boxextent (StaticMesh|GetBounds _asstatic_mesh))) "\",") (Utilities|String|Append " sphere_radius = " (Utilities|String|ToString(Float) (.sphereradius (StaticMesh|GetBounds _asstatic_mesh)))) " }, ")))
        (:CastFailed
          (return "")))
      (else
        _)))
  (return ""))

(fn FVectortoVectorString
  (params (InVec :type Vector))
  (return (Utilities|String|Append "Vector(" (Utilities|String|Replace (Utilities|String|Replace (Utilities|String|Replace (Utilities|String|Replace (Utilities|String|ToString(Vector) InVec) "X=") "Y=") "Z=") " " ", ") ")")))

(fn InternalGenerateMaps
  (TOMLGeneration|Assets|FetchAssetField (Variables|Assets|GetMaps) "maps" "maps")
  (return))

(fn InternalGenerateBlueprints
  (bind _returnvalue (TOMLGeneration|Assets|GenerateBlueprintsArray))
  (TOMLGeneration|Assets|FetchAssetField _returnvalue "blueprints" "blueprints")
  (return))

(fn GenerateAll
  (Variables|TOMLGeneration|SetGenerated "")
  (TOMLGeneration|Assets|CallAllGenerate)
  (Utility|MakeFinalGeneratedString))

(fn GenerateBlueprints
  (Variables|TOMLGeneration|SetGenerated "")
  (TOMLGeneration|Assets|Internal|InternalGenerateBlueprints)
  (Utility|MakeFinalGeneratedString))

(fn GenerateMaps
  (Variables|TOMLGeneration|SetGenerated "")
  (TOMLGeneration|Assets|Internal|InternalGenerateMaps)
  (Utility|MakeFinalGeneratedString))

(fn GenerateMaterials
  (Variables|TOMLGeneration|SetGenerated "")
  (TOMLGeneration|Assets|Internal|InternalGenerateMaterials)
  (Utility|MakeFinalGeneratedString))

(fn GenerateAnimations
  (Variables|TOMLGeneration|SetGenerated "")
  (TOMLGeneration|Assets|Internal|InternalGenerateAnimations)
  (Utility|MakeFinalGeneratedString))

(fn GenerateParticles
  (Variables|TOMLGeneration|SetGenerated "")
  (TOMLGeneration|Assets|Internal|InternalGenerateSounds)
  (Utility|MakeFinalGeneratedString))

(fn GenerateSounds
  (Variables|TOMLGeneration|SetGenerated "")
  (TOMLGeneration|Assets|Internal|InternalGenerateSounds)
  (Utility|MakeFinalGeneratedString))

(fn GenerateSkeletalMeshes
  (Variables|TOMLGeneration|SetGenerated "")
  (TOMLGeneration|Assets|Internal|InternalGenerateSkeletalMeshes)
  (Utility|MakeFinalGeneratedString))

(fn GenerateStaticMeshes
  (Variables|TOMLGeneration|SetGenerated "")
  (TOMLGeneration|Assets|Internal|InternalGenerateStaticMeshes)
  (Utility|MakeFinalGeneratedString))

(fn GenerateOthers
  (Variables|TOMLGeneration|SetGenerated "")
  (TOMLGeneration|Assets|Internal|InternalGenerateOthers)
  (Utility|MakeFinalGeneratedString))

(fn AddItemsArraySoftClass
  (params (Array :type Array%20of%20Object%20Soft%20Class%20References) (Add :type Array%20of%20Object%20Soft%20Class%20References))
  (for _array_element Add
    (Utilities|Array|Add Array _array_element))
  (return))