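; BP_ADKBlueprintUtilsLibrary is a utility function library that formats vectors and rotators as constructor-style strings, Vector(...) and Rotator(...).
; Each function takes the engine's ToString output and chains Replace calls to strip the axis labels, with a final Replace meant to comma-separate the values.
; The result is then wrapped in the type name and parentheses.
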(fn FVectortoVectorString
  (params (Vector :type Vector))
  (return (Utilities|String|Append "Vector(" (Utilities|String|Replace (Utilities|String|Replace (Utilities|String|Replace (Utilities|String|Replace (Utilities|String|ToString(Vector) Vector) "X=") "Y=") "Z=") " " ", ") ")")))

(fn FRotatortoRotatorString
  (params (Rotator :type Rotator))
  (return (Utilities|String|Append "Rotator(" (Utilities|String|Replace (Utilities|String|Replace (Utilities|String|Replace (Utilities|String|Replace (Utilities|String|ToString(Rotator) Rotator) "P=") "Y=") "R=") " " ", ") ")")))