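; Thumbnail generator that batch-exports JPG renders of every static and skeletal mesh under a searched /Game folder.
; Construction creates the scene capture's render target and finds the tagged stand-in static and skeletal mesh actors.
; Run swaps each mesh onto its stand-in, frames it from bounds, waits briefly, then exports to disk, optionally mirroring subfolders.
; Stop halts the loop between assets.
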(event Custom|RenderToDisk
  (params (FileName :type String) (FolderName :type String))
  (Class|ImageWriteBlueprintLibrary|ExporttoDisk (Variables|Default|GetRenderTarget) (Utilities|String|Append (Variables|Default|GetOutputFolderRaw) "/" (Utilities|String|SelectString (Utilities|String|Append FolderName "/" FileName) FileName (Variables|Default|GetbCreateSubfolders))) (Utilities|Struct|MakeImageWriteOptions "JPG" (delegate Custom|CustomEvent_0) 0 true true)))

(event Custom|CustomEvent_0
  (params (NewParam :type Boolean)))

(event Custom|Run
  (params (OutputFolder :type String) (SearchFolder :type String) (bCreateSubfolders :type Boolean))
  (bind _rt_staticmesh (Variables|Default|GetRT_StaticMesh))
  (bind _rt_skeletalmesh (Variables|Default|GetRT_SkeletalMesh))
  (bind _staticmeshcomponent (Variables|/Script/Engine.StaticMeshActor|GetStaticMeshComponent _rt_staticmesh))
  (bind _skeletalmeshcomponent (Variables|/Script/Engine.SkeletalMeshActor|GetSkeletalMeshComponent _rt_skeletalmesh))
  (Variables|Default|SetSearchFolder SearchFolder)
  (Variables|Default|SetOutputFolderRaw OutputFolder)
  (Variables|Default|SetbCreateSubfolders bCreateSubfolders)
  (Variables|Default|SetCurrentCount 0)
  (Variables|Default|SetbStop false)
  (bind _outassetdata (Class|AssetRegistry|GetAssetsbyPath (Class|AssetRegistryHelpers|GetAssetRegistry) (Utilities|String|StringToName (Utilities|String|Append "/Game/" (Variables|Default|GetSearchFolder))) true false))
  (if (and (< (Variables|Default|GetCurrentCount) (Utilities|Array|Length _outassetdata)) (not (Variables|Default|GetbStop))) :!label _label
    (if (and (not (Class|AssetRegistryHelpers|IsRedirector (Utilities|Array|Get(acopy) _outassetdata (Variables|Default|GetCurrentCount)))) (Class|AssetRegistryHelpers|IsValid (Utilities|Array|Get(acopy) _outassetdata (Variables|Default|GetCurrentCount))))
      (if (Utilities|Enum|Equal(Enum) (Utilities|GetClassDisplayName (Utilities|GetClass (Class|AssetRegistryHelpers|GetAsset (Utilities|Array|Get(acopy) _outassetdata (Variables|Default|GetCurrentCount))))) "StaticMesh")
        (Components|StaticMesh|SetStaticMesh _staticmeshcomponent (.AsStatic%20Mesh (Utilities|Casting|CastToStaticMesh (Class|AssetRegistryHelpers|GetAsset (Utilities|Array|Get(acopy) _outassetdata (Variables|Default|GetCurrentCount))))))
        (Variables|Default|SetBounds (StaticMesh|GetBounds (.AsStatic%20Mesh (Utilities|Casting|CastToStaticMesh (Class|AssetRegistryHelpers|GetAsset (Utilities|Array|Get(acopy) _outassetdata (Variables|Default|GetCurrentCount)))))))
        (Variables|Default|SetRT_Actor _rt_staticmesh)
        (Class|SkinnedMeshComponent|SetSkeletalMesh _skeletalmeshcomponent 0 true)
        (Transformation|SetActorLocation (Variables|Default|GetRT_Actor) (Math|Vector|MakeVector 0.0 0.0 (- (.z (.boxextent (Variables|Default|GetBounds))) (.Z (Math|Vector|BreakVector (.origin (Variables|Default|GetBounds)))))) false false :!label _label_2)
        (Transformation|SetActorLocation (+ (* (Transformation|GetActorForwardVector) (* (Math|Float|Max(Float) (* (.sphereradius (Variables|Default|GetBounds)) 2.0) 3e+01) -2.0)) (.origin (Variables|Default|GetBounds)) (Math|Vector|MakeVector 0.0 0.0 (- (.z (.boxextent (Variables|Default|GetBounds))) (.Z (Math|Vector|BreakVector (.origin (Variables|Default|GetBounds))))))) false false)
        (Utilities|FlowControl|Delay 0.05)
        (CallFunction|RendertoDisk (Utilities|GetDisplayName (Class|AssetRegistryHelpers|GetAsset (Utilities|Array|Get(acopy) _outassetdata (Variables|Default|GetCurrentCount)))) (Utilities|String|Replace (Utilities|String|Replace (Class|KismetSystemLibrary|GetPathName (Class|AssetRegistryHelpers|GetAsset (Utilities|Array|Get(acopy) _outassetdata (Variables|Default|GetCurrentCount)))) (Utilities|String|Append "/Game/" (Variables|Default|GetSearchFolder))) (Utilities|String|Append (Utilities|GetDisplayName (Class|AssetRegistryHelpers|GetAsset (Utilities|Array|Get(acopy) _outassetdata (Variables|Default|GetCurrentCount)))) "." (Utilities|GetDisplayName (Class|AssetRegistryHelpers|GetAsset (Utilities|Array|Get(acopy) _outassetdata (Variables|Default|GetCurrentCount)))))))
        (elif (Utilities|Enum|Equal(Enum) (Utilities|GetClassDisplayName (Utilities|GetClass (Class|AssetRegistryHelpers|GetAsset (Utilities|Array|Get(acopy) _outassetdata (Variables|Default|GetCurrentCount))))) "SkeletalMesh")
          (Class|SkinnedMeshComponent|SetSkeletalMesh _skeletalmeshcomponent (.AsSkeletal%20Mesh (Utilities|Casting|CastToSkeletalMesh (Class|AssetRegistryHelpers|GetAsset (Utilities|Array|Get(acopy) _outassetdata (Variables|Default|GetCurrentCount))))) true)
          (Variables|Default|SetBounds (StaticMesh|GetBounds (.AsSkeletal%20Mesh (Utilities|Casting|CastToSkeletalMesh (Class|AssetRegistryHelpers|GetAsset (Utilities|Array|Get(acopy) _outassetdata (Variables|Default|GetCurrentCount)))))))
          (Variables|Default|SetRT_Actor _rt_skeletalmesh)
          (Components|StaticMesh|SetStaticMesh _staticmeshcomponent 0)
          (goto _label_2)
          (else
            _))))
    (Math|Integer|IncrementInt (Variables|Default|GetCurrentCount)
      (:%20%20
        (goto _label)))
    (else
      (Development|PrintString "Finished!"))))

(event Custom|Stop
  (Variables|Default|SetbStop true))

(fn ConstructionScript
  (bind _returnvalue (Rendering|CreateRenderTarget2D 256 256 "RTF_RGBA8" "(R=0.000000,G=0.000000,B=0.000000,A=0.000000)"))
  (bind _output_get (Variables|Default|SetRenderTarget _returnvalue))
  (Variables|/Script/Engine.TextureRenderTarget|SetTargetGamma _output_get 2.2)
  (Variables|/Script/Engine.SceneCaptureComponent2D|SetTextureTarget (Variables|Default|GetSceneCaptureComponent2D) _output_get)
  (Utilities|FlowControl|Sequence
    (:then_0
      (bind _outactors (Actor|GetAllActorsOfClasswithTag "/Script/Engine.StaticMeshActor" "RT_StaticMesh"))
      (if (Utilities|Array|IsValidIndex _outactors)
        (Variables|Default|SetRT_StaticMesh (Utilities|Array|Get(acopy) _outactors))))
    (:then_1
      (bind _outactors_2 (Actor|GetAllActorsOfClasswithTag "/Script/Engine.SkeletalMeshActor" "RT_SkeletalMesh"))
      (if (Utilities|Array|IsValidIndex _outactors_2)
        (Variables|Default|SetRT_SkeletalMesh (Utilities|Array|Get(acopy) _outactors_2))))))