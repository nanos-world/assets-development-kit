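; Function library for Nanos World that locates the directional light component acting as the level's sun.
; GetSunLightComponent tries three sources in priority order: a DirectionalLight actor, a SunSky actor, then any actor tagged "Sun" with a directional light component.
; It takes only the first actor of each search and returns the component with a Found flag, which is false when no source matches.
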(fn GetSunLightComponent
  (bind _outactors (Actor|GetAllActorsOfClass 0 "/Script/Engine.DirectionalLight"))
  (if (Utilities|Array|IsValidIndex _outactors)
    (return (Variables|/Script/Engine.Light|GetLightComponent (Utilities|Array|Get(acopy) _outactors)) true)
    (else
      (bind _outactors_2 (Actor|GetAllActorsOfClass 0 "/SunPosition/SunSky.SunSky_C"))
      (if (Utilities|Array|IsValidIndex _outactors_2)
        (return (Variables|/SunPosition/SunSky.SunSky_C|GetDirectionalLight (Utilities|Array|Get(acopy) _outactors_2)) true)
        (else
          (bind _outactors_3 (Actor|GetAllActorsOfClasswithTag 0 "/Script/Engine.Actor" "Sun"))
          (if (Utilities|Array|IsValidIndex _outactors_3)
            (Utilities|IsValid (Actor|GetComponentbyClass (Utilities|Array|Get(acopy) _outactors_3) "/Script/Engine.DirectionalLightComponent")
              (:Is%20Valid
                (return (Actor|GetComponentbyClass (Utilities|Array|Get(acopy) _outactors_3) "/Script/Engine.DirectionalLightComponent") true))
              (:Is%20Not%20Valid
                _)))
          (return 0 false))))))